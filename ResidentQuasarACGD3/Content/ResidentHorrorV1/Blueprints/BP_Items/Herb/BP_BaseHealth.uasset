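; BP_BaseHealth is a usable healing item in the Herb items folder that restores the player character's health.
; UseItem checks the HealthComponent's current HP against a hardcoded 99 threshold.
; At or below it, the item heals by the cure amount from its interact data asset, then runs the parent UseItem.
; Otherwise it plays the inventory fail sound and shows the WBP_HpMax widget without calling the parent.
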(event `self.ReceiveBeginPlay`
  (`parent.ReceiveBeginPlay`))

(fn `UseItem`
  (returns (Sucess :type Boolean))
  (if (<= (`/Game/ResidentHorrorV1/Blueprints/BP_HealthComponent/HealthComponent.Current Hp` (`/Game/ResidentHorrorV1/Character/BP_Character/BP_Resident_HorrorV1.HealthComponent` (`/Game/ResidentHorrorV1/Blueprints/BP_FunctionLibray/BPFL_LibrayCharacter.My character Resident Horror`))) 99.0)
    (`/Game/ResidentHorrorV1/Blueprints/BP_HealthComponent/HealthComponent.Take healing` (`/Game/ResidentHorrorV1/Character/BP_Character/BP_Resident_HorrorV1.HealthComponent` (`/Game/ResidentHorrorV1/Blueprints/BP_FunctionLibray/BPFL_LibrayCharacter.My character Resident Horror`)) (`/Game/ResidentHorrorV1/Blueprints/BP_Inventory/DA_BaseInteract.How much does it cure?` (`.DA_BaseInteract_112_E5D63A474E86D51C38EA9ABF9499DC91` (break `/Game/ResidentHorrorV1/Blueprints/BP_Inventory/S_Item_Structure` (`.ItemStructure_3_D962DD8B4106829899F7C99F3F34F837` (break `/Game/ResidentHorrorV1/Blueprints/BP_Inventory/S_SlotStruct` (`self.S ItemStrucuture`)))))))
    (bind _sucess (`parent.UseItem`))
    (return _sucess)
    (else
      (`GameplayStatics.PlaySound2D` (`/Game/ResidentHorrorV1/Blueprints/BP_CustomDataAssets/Base/DA_InventoryCustom.Sound Fail` (`self.DA InventoryCustom`)) 1.0 1.0 0.0 null null)
      (bind _returnvalue (`|CreateWidget` "/Game/ResidentHorrorV1/Blueprints/WBP/WBP_Interact/WBP_HpMax.WBP_HpMax_C"))
      (`UserWidget.AddToViewport` _returnvalue 0))))

(fn `UserConstructionScript`
  (`parent.UserConstructionScript`))